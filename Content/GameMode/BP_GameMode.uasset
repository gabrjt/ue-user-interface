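; Game mode that initializes the friend subsystem and simulates friends going online and offline.
; On BeginPlay it loads friends from a data table, binds to the subsystem's update event and hands a FriendSubsystem reference to BP_FriendHUD.
; A looping timer periodically inverts every friend's connected state through the subsystem, and each update event prints the nickname and new status.
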(event Custom|Event%20FriendUpdated
  (params (FriendData :type Friend%20Data%20Structure))
  (Development|PrintString (Class|KismetStringLibrary|BuildStringBool (.nickname FriendData) " " (.bisconnected FriendData))))

(event Custom|Event%20UpdateFriend
  (bind _returnvalue (Subsystems|GetFriendSubsystem))
  (for _array_element (Class|FriendService|GetFriends _returnvalue)
    (Class|FriendSubsystem|SetFriendIsConnected _returnvalue (.userid _array_element) (not (.bisconnected _array_element)))))

(event EventBeginPlay
  (bind _returnvalue (Subsystems|GetFriendSubsystem))
  (Utilities|FlowControl|Sequence
    (:then_0
      (Class|FriendSubsystem|LoadFriends _returnvalue "/Game/Data/DT_Friends.DT_Friends")
      (EventDispatchers|BindEventtoOnFriendUpdatedBP _returnvalue (delegate Custom|Event%20FriendUpdated)))
    (:then_1
      (bind _asbp_friend_hud (Utilities|Casting|CastToBP_FriendHUD (HUD|GetHUD (Game|GetPlayerController 0))))
      (Variables|/Script/UserInterface.FriendHUD|SetFriendSubsystemClass _asbp_friend_hud "/Script/UserInterface.FriendSubsystem"))
    (:then_2
      (Utilities|Time|SetTimerbyEvent (delegate Custom|Event%20UpdateFriend) 3.0 true true))))

(fn ConstructionScript)